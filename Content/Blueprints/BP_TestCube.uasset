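; BP_TestCube is a test actor that implements a movement interface for direction and speed.
; Move offsets the root component's world position by the normalized Direction times MoveSpeed, using a swept move without delta-time scaling.
; SetSpeed and SetDirection store their values, but Move ignores the stored direction.
; GetSpeed and GetDirection return zero instead of the stored values, and BeginPlay, Tick and overlap events are empty.
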(event `self.Move`
  (params (direction :type "Vector Structure"))
  (bind _defaultsceneroot (`self.DefaultSceneRoot`))
  ;[0.08854 0.08854 0.08854] インターフェースからの移動
  (`SceneComponent.K2_SetWorldLocation` _defaultsceneroot (+ (* (`KismetMathLibrary.Normal` direction) (`self.MoveSpeed`)) (`SceneComponent.K2_GetComponentLocation` _defaultsceneroot)) true false))

(event `self.SetSpeed`
  (params (speed :type "Float (single-precision)"))
  ;[0.0625 0.0625 0.0625] インターフェースのセッタ
  (set `self.MoveSpeed` speed))

(event `self.SetDirection`
  (params (direction :type "Vector Structure"))
  ;[0.0625 0.0625 0.0625] インターフェースのセッタ
  (set `self.MoveDIrection` direction))

(fn `GetDirection`
  (returns (ReturnValue :type "Vector Structure"))
  (return (0.0 0.0 0.0)))

(fn `GetSpeed`
  (returns (ReturnValue :type "Float (single-precision)"))
  (return 0.0))

(fn `UserConstructionScript`)