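; Actor component that drives its owner automatically along a route of BP_MovePoint actors placed in the level.
; On BeginPlay it gathers the points targeting its owner, starts at the one flagged as entry and binds to their arrival events.
; Each arrival supplies the next destination, or sets speed to zero when none follows.
; Tick sends the owner the unnormalized vector toward the current point through a move message.
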(event `self.ReceiveBeginPlay`
  (bind _distination (`self.Distination`))
  (set `self.ParentActor` (`self.GetOwner`))
  (bind _result (`self.FindMovePoints`))
  (set `self.MovePoints` _result)
  (bind _result_2 (`self.FindEntryPoint`))
  (set `self.Distination` _result_2)
  (add `/Game/Blueprints/BP_MovePoint.OnPointArrival` (`self.MovePoints`) (delegate `CustomEvent`))
  (if (`KismetSystemLibrary.IsValid` _distination)
    (set `/Game/Blueprints/BP_MovePoint.TargetDistination` _distination _distination)))

(event `CustomEvent`
  (params (Next :type "/Game/Blueprints/BP_MovePoint Object Reference"))
  (if (`KismetSystemLibrary.IsValid` Next)
    (bind _output_get (set `self.Distination` Next))
    (set `/Game/Blueprints/BP_MovePoint.TargetDistination` _output_get _output_get)
    (else
      (message `/Game/Interfaces/BI_Moveable.SetSpeed` (`self.ParentActor`) 0.0))))

(event `self.ReceiveTick`
  (params (DeltaSeconds :type "Float (single-precision)"))
  (if (`KismetSystemLibrary.IsValid` (`self.Distination`))
    (bind _resultvector (`self.GetPointToVector` (`self.Distination`)))
    (message `/Game/Interfaces/BI_Moveable.Move` (`self.ParentActor`) _resultvector)))

(fn `FindEntryPoint`
  (returns (Result :type "/Game/Blueprints/BP_MovePoint Object Reference"))
  (locals (ResultPoint :type "/Game/Blueprints/BP_MovePoint Object Reference"))
  (for _array_element (`self.MovePoints`)
    (if (`/Game/Blueprints/BP_MovePoint.EntryPoint` _array_element)
      (set `local.ResultPoint` _array_element)
      (break)))
  (return (`local.ResultPoint`)))

(fn `FindMovePoints`
  (returns (Result :type "Array of /Game/Blueprints/BP_MovePoint Object Reference"))
  (locals (ResultPoints :type "Array of /Game/Blueprints/BP_MovePoint Object Reference"))
  (bind _outactors (`GameplayStatics.GetAllActorsOfClass` "/Game/Blueprints/BP_MovePoint.BP_MovePoint_C"))
  (for _array_element _outactors
    (if (== (`/Game/Blueprints/BP_MovePoint.TargetActor` _array_element) (`self.ParentActor`))
      (`KismetArrayLibrary.Array_Add` (`local.ResultPoints`) _array_element)))
  (return (`local.ResultPoints`)))

(fn `GetPointToVector`
  (params (Point :type "/Game/Blueprints/BP_MovePoint Object Reference"))
  (returns (ResultVector :type "Vector Structure"))
  (return (- (`Actor.K2_GetActorLocation` Point) (`Actor.K2_GetActorLocation` (`self.ParentActor`)))))