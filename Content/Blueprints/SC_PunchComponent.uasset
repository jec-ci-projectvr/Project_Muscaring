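; Scene component that performs a punch hit check and triggers a field effect where the punch lands.
; HitTrace fires OnPunch, then sphere-traces along the component's forward vector using Length and Radius, with one-frame debug drawing.
; On a hit, it spawns a short-lived BP_MasterField at the impact point, calls CETrigger on it and destroys it immediately.
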(fn `HitTrace`
  (bind (_returnvalue_location _returnvalue_rotation) (`KismetMathLibrary.BreakTransform` (`self.K2_GetComponentToWorld`)))
  (`self.OnPunch`)
  (bind (_outhit _returnvalue) (`KismetSystemLibrary.SphereTraceSingle` :`Start` _returnvalue_location :`End` (+ _returnvalue_location (* (`KismetMathLibrary.GetForwardVector` _returnvalue_rotation) (`self.Length`))) :`Radius` (`self.Radius`) :`TraceChannel` "TraceTypeQuery3" :`DrawDebugType` "ForOneFrame"))
  (if _returnvalue
    (bind _returnvalue_2 (`|SpawnActorFromClass` "/Game/Blueprints/BP_MasterField.BP_MasterField_C" (`KismetMathLibrary.MakeTransform` (`.ImpactPoint` (`GameplayStatics.BreakHitResult` _outhit))) "Undefined" "MultiplyWithRoot" null null))
    (`/Engine/EditorResources/FieldNodes/FS_MasterField.CE_Trigger` _returnvalue_2)
    (`Actor.K2_DestroyActor` _returnvalue_2)))