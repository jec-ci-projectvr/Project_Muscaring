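; TestCube is a test actor, apparently a cube, that is moved through an interface.
; Move normalizes the passed direction, scales it by MoveSpeed and offsets the root's world location without sweep or delta time, so each call is a fixed step.
; Setters and getters expose the stored speed and direction, but Move uses only its Direction argument, not the stored direction.
; BeginPlay, overlap, Tick and the construction script are empty.
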(event `/Game/Interfaces/IMoveable.Move`
  (params (Direction :type "Vector Structure"))
  (bind _defaultsceneroot (`self.DefaultSceneRoot`))
  ;[0.08854 0.08854 0.08854] インターフェースからの移動
  (`SceneComponent.K2_SetWorldLocation` _defaultsceneroot (+ (* (`KismetMathLibrary.Normal` Direction) (`self.MoveSpeed`)) (`SceneComponent.K2_GetComponentLocation` _defaultsceneroot)) false false))

(event `/Game/Interfaces/IMoveable.SetSpeed`
  (params (Speed :type "Float (double-precision)"))
  ;[0.0625 0.0625 0.0625] インターフェースのセッタ
  (set `self.MoveSpeed` Speed))

(event `/Game/Interfaces/IMoveable.SetDirection`
  (params (Direction :type "Vector Structure"))
  ;[0.0625 0.0625 0.0625] インターフェースのセッタ
  (set `self.MoveDIrection` Direction))

(fn `GetDirection`
  (returns (Direction :type "Vector Structure"))
  (return (`self.MoveDirection`)))

(fn `GetSpeed`
  (returns (Speed :type "Float (double-precision)"))
  (return (`self.MoveSpeed`)))

(fn `UserConstructionScript`)