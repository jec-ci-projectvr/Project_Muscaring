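; Breakable entrance door actor that registers Chaos break events on its geometry collection as hits toward being broken.
; On BeginPlay it rebinds the component's break event to a handler.
; Each accepted break increments a hit count, updates the broken state against the required count, and plays a sound at the break location.
; A timeline acts as a cooldown, ignoring further breaks until it finishes.
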(event `self.ReceiveBeginPlay`
  (bind _geometrycollectioncomponent (`self.GeometryCollectionComponent`))
  (clear `GeometryCollectionComponent.OnChaosBreakEvent` _geometrycollectioncomponent)
  (add `GeometryCollectionComponent.OnChaosBreakEvent` _geometrycollectioncomponent (delegate `OnChaosBreakEvent_イベント`)))

(event `OnChaosBreakEvent_イベント`
  (params (BreakEvent :type "ChaosBreakEvent Structure (by ref)"))
  (if (not (`self.IsAttacked`))
    (set `self.IsAttacked` true)
    (`/Engine/EditorBlueprintResources/StandardMacros.IncrementInt` (`self.HitNum`)
      (:`  `
        (`self.SetBreaked` (>= (`self.HitNum`) (`self.HitNeedCount`)))
        (`GameplayStatics.PlaySoundAtLocation` (`self.breakSound`) BreakEvent_Location (struct) 1.0 1.0 0.0 null null null null)
        (`Timeline|タイムライン` :!via `PlayFromStart`
          (:`Finished`
            (set `self.IsAttacked` false)))))))

(fn `IsResumeTrigger`
  (returns (ReturnValue :type Boolean))
  (return false))

(fn `UserConstructionScript`)