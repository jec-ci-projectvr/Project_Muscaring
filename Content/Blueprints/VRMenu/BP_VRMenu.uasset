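; VR menu actor that loads MapLevel through a progress bar driven by the player character's LevelOpen flag.
; While the flag is set, Tick plays a timeline that fills the WB_VRMenu bar, reversing it if the flag clears before completion.
; A full bar starts, once only, a non-blocking hidden stream load and a fade sequence, whose finish opens the level.
; The OpenLevel event caches the VRCharacter reference that Tick polls.
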(event `self.ReceiveTick`
  (params (DeltaSeconds :type "Float (single-precision)"))
  (bind _textrender (`self.TextRender`))
  (bind _sequenceplayer (`LevelSequenceActor.SequencePlayer` (`self.FadeSequence`)))
  (if (`/Game/Blueprints/VRCharacter.LevelOpen` (stale `OpenLevel` _asvrcharacter))
    (`TextRenderComponent.K2_SetText` _textrender (`self.LowdingText`))
    (bind (_direction _newtrack_1) (`Timeline|Timeline_OpenLevel` :!label _label)
      (:`Update`
        (set `self.Percent` _newtrack_1)
        (bind _aswb_vrmenu (cast `/Game/Blueprints/VRMenu/WB_VRMenu` (`WidgetComponent.GetUserWidgetObject` (`self.Widget`))))
        (`ProgressBar.SetPercent` (`/Game/Blueprints/VRMenu/WB_VRMenu.ProgressBar_VRMenu` _aswb_vrmenu) (`self.Percent`)))
      (:`Finished`
        (if (== (`self.Percent`) 1.0)
          (`/Engine/EditorBlueprintResources/StandardMacros.DoOnce` false
            (:`Completed`
              (add `MovieSceneSequencePlayer.OnFinished` _sequenceplayer (delegate `CustomEvent`))
              (`GameplayStatics.LoadStreamLevel` "MapLevel")
              (`MovieSceneSequencePlayer.Play` _sequenceplayer))))))
    (elif (not (== (`self.Percent`) 1.0))
      (`TextRenderComponent.K2_SetText` _textrender (`self.StandText`))
      (goto _label :!via `Reverse`))))

(event `OpenLevel`
  (bind _asvrcharacter (cast `/Game/Blueprints/VRCharacter` (`GameplayStatics.GetPlayerCharacter` 0))))

(event `CustomEvent`
  (`GameplayStatics.OpenLevel` "MapLevel"))

(fn `UserConstructionScript`)