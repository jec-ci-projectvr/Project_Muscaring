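; Actor component that plays footstep sounds for its owner, varying them by the ground's surface type.
; A Delay on Tick paces steps by PlaySpan, and each step plays only while IsSoundPlay is set.
; A visibility trace from the owner's location to its scaled, negated up vector (not offset by location) maps Default, Tatami or Dirt to an index.
; That index sets the cue's GroundType parameter before playback at the hit location.
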(event `self.ReceiveBeginPlay`
  (set `self.Owner` (`self.GetOwner`))
  (set `self.WalkSoundCue` "/Game/Sound/WalkGround.WalkGround"))

(event `self.ReceiveTick`
  (params (DeltaSeconds :type "Float (single-precision)"))
  (`KismetSystemLibrary.Delay` (`self.PlaySpan`))
  (if (`self.IsSoundPlay`)
    (bind (_result _location) (`self.TraceGround`))
    (`self.PlayStepSound` _result _location)))

(fn `PlayStepSound`
  (params (SoundIndex :type Integer) (Location :type "Vector Structure"))
  (message `AudioParameterControllerInterface.SetIntParameter` (`self.WalkSoundCue`) "GroundType" SoundIndex)
  (`GameplayStatics.PlaySoundAtLocation` (`self.WalkSoundCue`) Location (struct) 1.0 1.0 0.0 null null null null))

(fn `TraceGround`
  (returns (Result :type Integer) (Location :type "Vector Structure"))
  (locals (sound :type "SoundBase Object Reference"))
  (bind _owner (`self.Owner`))
  (bind _outhit (`KismetSystemLibrary.LineTraceSingle` (`Actor.K2_GetActorLocation` _owner) (* (`Actor.GetActorUpVector` _owner) -2.0) "TraceTypeQuery1"))
  (bind (_bblockinghit _binitialoverlap _time _distance _location _impactpoint _normal _impactnormal _physmat) (`GameplayStatics.BreakHitResult` _outhit))
  (return (select `EPhysicalSurface` (`PhysicalMaterial.SurfaceType` _physmat) :`SurfaceType1` 1 :`SurfaceType2` 2) _location))