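; BP_LoadTriggerBox is a trigger volume that moves the player to another level after a fade sequence.
; The first overlap by player 0's pawn starts a non-blocking, hidden stream load of LoadLevelName and plays FadeSequence.
; When the sequence player finishes, a bound event opens that same level by name, making it a full level change rather than revealing the streamed one.
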(event `self.CollisionComponent.OnComponentBeginOverlap`
  (params (OverlappedComponent :type "PrimitiveComponent Object Reference") (OtherActor :type "Actor Object Reference") (OtherComp :type "PrimitiveComponent Object Reference") (OtherBodyIndex :type Integer) (bFromSweep :type Boolean) (SweepResult :type "HitResult Structure (by ref)"))
  (bind _sequenceplayer (`LevelSequenceActor.SequencePlayer` (`self.FadeSequence`)))
  (if (== OtherActor (`GameplayStatics.GetPlayerPawn` 0))
    (`/Engine/EditorBlueprintResources/StandardMacros.DoOnce` false
      (:`Completed`
        (add `MovieSceneSequencePlayer.OnFinished` _sequenceplayer (delegate `OpenLevel`))
        (`GameplayStatics.LoadStreamLevel` (`self.LoadLevelName`))
        (`MovieSceneSequencePlayer.Play` _sequenceplayer)))))

(event `OpenLevel`
  (`GameplayStatics.OpenLevel` (`self.LoadLevelName`)))

(fn `UserConstructionScript`)