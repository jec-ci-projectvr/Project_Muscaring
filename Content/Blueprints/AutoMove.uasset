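; AutoMove is a component that automatically steers its owning actor along a route of MovePoint actors.
; On BeginPlay it gathers the MovePoints that target its owner, starts toward the one flagged as entry point and binds to their arrival events.
; Each arrival event supplies the next destination.
; Every Tick it passes the unnormalized offset to that destination through a Move message, leaving the movement itself to the owner.
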(event `self.ReceiveBeginPlay`
  (set `self.ParentActor` (`self.GetOwner`))
  (bind _result (`self.FindMovePoints`))
  (set `self.MovePoints` _result)
  (bind _result_2 (`self.FindEntryPoint`))
  (set `self.Distination` _result_2)
  (add `/Game/Blueprints/MovePoint.OnPointArrival` (`self.MovePoints`) (delegate `CustomEvent`)))

(event `CustomEvent`
  (params (Next :type "/Game/Blueprints/MovePoint Object Reference"))
  (set `self.Distination` Next))

(event `self.ReceiveTick`
  (params (DeltaSeconds :type "Float (single-precision)"))
  (if (`KismetSystemLibrary.IsValid` (`self.Distination`))
    (bind _resultvector (`self.GetPointToVector` (`self.Distination`)))
    (message `/Game/Interfaces/IMoveable.Move` (`self.ParentActor`) _resultvector)))

(fn `FindEntryPoint`
  (returns (Result :type "/Game/Blueprints/MovePoint Object Reference"))
  (locals (ResultPoint :type "/Game/Blueprints/MovePoint Object Reference"))
  (for _array_element (`self.MovePoints`)
    (if (`/Game/Blueprints/MovePoint.EntryPoint` _array_element)
      (set `local.ResultPoint` _array_element)
      (break)))
  (return (`local.ResultPoint`)))

(fn `FindMovePoints`
  (returns (Result :type "Array of /Game/Blueprints/MovePoint Object Reference"))
  (locals (ResultPoints :type "Array of /Game/Blueprints/MovePoint Object Reference"))
  (bind _outactors (`GameplayStatics.GetAllActorsOfClass` "/Game/Blueprints/MovePoint.MovePoint_C"))
  (for _array_element _outactors
    (if (== (`/Game/Blueprints/MovePoint.TargetActor` _array_element) (`self.ParentActor`))
      (`KismetArrayLibrary.Array_Add` (`local.ResultPoints`) _array_element)))
  (return (`local.ResultPoints`)))

(fn `GetPointToVector`
  (params (Point :type "/Game/Blueprints/MovePoint Object Reference"))
  (returns (ResultVector :type "Vector Structure"))
  (return (- (`Actor.K2_GetActorLocation` Point) (`Actor.K2_GetActorLocation` (`self.ParentActor`)))))