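; Normal ghost character whose scare points drive its behavior state: Approach, Scare, Escape or Swoon.
; The player's FakeOut action and the first pawn sighting raise the points, then threshold checks pick the state and set walk speed.
; It forwards the state, the nearest BP_RestArea found at BeginPlay, and capsule overlap hits to its AI controller via messages.
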(event `self.ReceiveBeginPlay`
  (add `/Game/Blueprints/AC_PlayerAction.OnFakeOut` (`self.GetComponentByClass` (`GameplayStatics.GetPlayerPawn` 0) "/Game/Blueprints/AC_PlayerAction.AC_PlayerAction_C") (delegate `OnFakeOut_イベント`))
  ;[1 1 1] 最寄りの休憩所を設定
  (bind _outactors (`GameplayStatics.GetAllActorsOfClass` "/Game/Blueprints/BP_RestArea.BP_RestArea_C"))
  (for (_array_element _array_index) _outactors :!label _label
    (bind _returnvalue (`self.GetDistanceTo` _array_element self))
    (if (< _returnvalue (`self.MinimumDist`))
      (set `self.MinimumDist` _returnvalue)
      (bind _output_get (set `self.ReferenceRestArea` _array_element))
      (goto _label)))
  (message `/Game/Characters/Ghosts/AI/BPI_DeliveryGhostState.SendMostNearRestArea` (`AIBlueprintHelperLibrary.GetAIController` self) _output_get)
  (`KismetSystemLibrary.PrintString` (`KismetStringLibrary.Conv_IntToString` _array_index)))

(event `OnFakeOut_イベント`
  (bind _state (`self.State`))
  (bind _charactermovement (`self.CharacterMovement`))
  ;[1 1 1] 恐怖地と状態の制御
  (`KismetSystemLibrary.PrintString` "Neko")
  (set `self.ScarePoint` (+ (`self.ScarePoint`) 10))
  (bind _output_get (set `self.ScarePoint` (+ (`self.ScarePoint`) 1) :!label _label_2))
  (if (< _output_get 30)
    (set `self.State` "NewEnumerator1")
    (message `/Game/Characters/Ghosts/AI/BPI_DeliveryGhostState.SendGhostState` (`AIBlueprintHelperLibrary.GetAIController` self) _state :!label _label_3)
    ;[1 1 1] 状態ごとの移動速度の決定
    (switch `/Game/Characters/Ghosts/AI/EN_GhostState` _state
      (:`NewEnumerator1`
        (bind _output_get_2 (set `CharacterMovementComponent.MaxWalkSpeed` (`self.DefaultMoveSpeed_0`) _charactermovement))
        (`KismetSystemLibrary.PrintString` (`KismetStringLibrary.Conv_DoubleToString` _output_get_2)))
      (:`NewEnumerator2`
        (bind _output_get_3 (set `CharacterMovementComponent.MaxWalkSpeed` (/ (`self.DefaultMoveSpeed_0`) 2.0) _charactermovement))
        (`KismetSystemLibrary.PrintString` (`KismetStringLibrary.Conv_DoubleToString` _output_get_3)))
      (:`NewEnumerator3`
        (bind _output_get_4 (set `CharacterMovementComponent.MaxWalkSpeed` (`self.EscapeMoveSpeed`) _charactermovement))
        (`KismetSystemLibrary.PrintString` (`KismetStringLibrary.Conv_DoubleToString` _output_get_4)))
      (:`NewEnumerator4`
        (bind _output_get_5 (set `CharacterMovementComponent.MaxWalkSpeed` (`self.DefaultMoveSpeed_0`) _charactermovement))
        (`KismetSystemLibrary.PrintString` (`KismetStringLibrary.Conv_DoubleToString` _output_get_5))))
    (elif (< _output_get 60)
      (set `self.State` "NewEnumerator2")
      (goto _label_3)
      (elif (< _output_get 100)
        (set `self.State` "NewEnumerator3")
        (goto _label_3)
        (elif (>= _output_get 100)
          (set `self.State` "NewEnumerator4")
          (goto _label_3))))))

(event `self.PawnSensing.OnSeePawn`
  (params (Pawn :type "Pawn Object Reference"))
  ;[1 1 1] 恐怖地と状態の制御
  (if (not (`self.OnSeeOnce`))
    (set `self.OnSeeOnce` true)
    (goto _label_2)))

(event `self.CapsuleComponent.OnComponentBeginOverlap`
  (params (OverlappedComponent :type "PrimitiveComponent Object Reference") (OtherActor :type "Actor Object Reference") (OtherComp :type "PrimitiveComponent Object Reference") (OtherBodyIndex :type Integer) (bFromSweep :type Boolean) (SweepResult :type "HitResult Structure (by ref)"))
  (bind _charactermovement (`self.CharacterMovement`))
  (message `/Game/Characters/Ghosts/AI/BPI_DeliveryGhostState.SendHitInfo` (`AIBlueprintHelperLibrary.GetAIController` self) true)
  (`KismetSystemLibrary.PrintString` "Hit")
  (bind _output_get (set `CharacterMovementComponent.MaxWalkSpeed` (`CharacterMovementComponent.MaxWalkSpeed` _charactermovement) _charactermovement))
  (`KismetSystemLibrary.PrintString` (`KismetStringLibrary.Conv_DoubleToString` _output_get)))

(fn `UserConstructionScript`)