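; AI controller for the normal ghost that runs the BT_NormalGhost behavior tree.
; On BeginPlay it starts the tree and writes its controlled pawn and the player pawn to the blackboard as SelfActor and Target.
; Events for ghost state, nearest rest area and hit info copy the received values into the GhostState, RestArea and Hit blackboard keys.
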(event `self.ReceiveBeginPlay`
  (`self.RunBehaviorTree` "/Game/Characters/Ghosts/AI/BT_NormalGhost.BT_NormalGhost")
  ;[1 1 1] 自身のキー設定
  (`BlackboardComponent.SetValueAsObject` (`self.Blackboard`) "SelfActor" (`self.K2_GetPawn`))
  ;[1 1 1] プレイヤーのキー設定
  (`BlackboardComponent.SetValueAsObject` (`self.Blackboard`) "Target" (`GameplayStatics.GetPlayerPawn` 0)))

(event `/Game/Characters/Ghosts/AI/BPI_DeliveryGhostState.SendGhostState`
  (params (State :type "/Game/Characters/Ghosts/AI/EN_GhostState Enum (by ref)" :default "NewEnumerator0"))
  (`BlackboardComponent.SetValueAsEnum` (`self.Blackboard`) "GhostState" State))

(event `/Game/Characters/Ghosts/AI/BPI_DeliveryGhostState.SendMostNearRestArea`
  (params (RestArea :type "/Game/Blueprints/BP_RestArea Object Reference"))
  (`BlackboardComponent.SetValueAsObject` (`self.Blackboard`) "RestArea" RestArea))

(event `/Game/Characters/Ghosts/AI/BPI_DeliveryGhostState.SendHitInfo`
  (params (IsHit :type Boolean))
  (`BlackboardComponent.SetValueAsBool` (`self.Blackboard`) "Hit" IsHit))

(fn `UserConstructionScript`)