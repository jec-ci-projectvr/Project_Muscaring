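; BP_EndingGhost is an ending actor that plays a jingle, moves steadily, and triggers a level change after travelling a set distance.
; Tick applies a fixed local offset per frame, unscaled by delta time, until world Y exceeds the start plus LoadInterval.
; A DoOnce then starts a hidden, non-blocking stream load of LoadLevelName and plays FadeSequence, whose finish event opens that level by name.
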(event `self.ReceiveBeginPlay`
  (bind (_returnvalue_x _returnvalue_y) (`KismetMathLibrary.BreakVector` (`self.K2_GetActorLocation`)))
  (set `self.EndLocationY` (+ _returnvalue_y (`self.LoadInterval`)))
  (`GameplayStatics.PlaySound2D` "/Game/Ending/EndingJingle.EndingJingle" 1.0 1.0 0.0 null null))

(event `self.ReceiveTick`
  (params (DeltaSeconds :type "Float (single-precision)"))
  (bind (_returnvalue_x _returnvalue_y) (`KismetMathLibrary.BreakVector` (`self.K2_GetActorLocation`)))
  (bind _sequenceplayer (`LevelSequenceActor.SequencePlayer` (`self.FadeSequence`)))
  (`self.K2_AddActorLocalOffset` (`self.MoveSpeed`))
  (if (> _returnvalue_y (`self.EndLocationY`))
    (`/Engine/EditorBlueprintResources/StandardMacros.DoOnce` false
      (:`Completed`
        (add `MovieSceneSequencePlayer.OnFinished` _sequenceplayer (delegate `OpenLevel`))
        (`GameplayStatics.LoadStreamLevel` (`self.LoadLevelName`))
        (`MovieSceneSequencePlayer.Play` _sequenceplayer)))))

(event `OpenLevel`
  (`GameplayStatics.OpenLevel` (`self.LoadLevelName`)))

(fn `UserConstructionScript`)